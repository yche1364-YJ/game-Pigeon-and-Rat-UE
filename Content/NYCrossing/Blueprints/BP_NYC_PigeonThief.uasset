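; BP_NYC_PigeonThief is a thief that swoops at the player's pigeon to steal the food it carries.
; Tick runs idle, dive and escape modes; each new pickup grants as many attempts as pickups so far, launched after random delays.
; The lerped, sine-arced dive raises Warn and partly tracks the player; a close finish calls Steal and sets the food mesh.
; An unconnected copy of the Tick logic, without attempt counting, never runs.
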(event `self.ReceiveBeginPlay`
  (set `self.Mode` 0)
  (set `self.Pickups` 0)
  (set `self.Attempts` 0)
  (set `self.LastCarry` 0)
  (set `self.NextTime` (+ (`KismetSystemLibrary.GetGameTimeInSeconds`) 4.0))
  (`SceneComponent.SetVisibility` (`self.Model`) false true))

(event `self.ReceiveTick`
  (params (DeltaSeconds :type "Float (single-precision)"))
  (bind _returnvalue (`KismetSystemLibrary.GetGameTimeInSeconds`))
  (bind _returnvalue_2 (`self.K2_GetActorLocation`))
  (bind _food (`self.Food`))
  (bind _returnvalue_3 (`KismetMathLibrary.DegSin` (* _returnvalue 900.0)))
  (bind _returnvalue_4 (+ (`self.T`) (/ DeltaSeconds 1.6)))
  (bind _returnvalue_5 (+ (`self.T`) (/ DeltaSeconds 2.0)))
  (bind _returnvalue_6 (`KismetMathLibrary.VLerp` (`self.P0`) (`self.P1`) _returnvalue_4))
  (bind _asbp_nyc_pigeon (cast `/Game/NYCrossing/Blueprints/BP_NYC_Pigeon` (`GameplayStatics.GetPlayerPawn` 0)))
  (bind _state (`/Game/NYCrossing/Blueprints/BP_NYC_Pigeon.State` _asbp_nyc_pigeon))
  (if (and (!= _state 1) (!= _state 2))
    (set `self.Pickups` 0)
    (set `self.Attempts` 0))
  (bind _carrying (`/Game/NYCrossing/Blueprints/BP_NYC_Pigeon.Carrying` _asbp_nyc_pigeon))
  (if (and (> _carrying 0) (== (`self.LastCarry`) 0))
    (set `self.Pickups` (+ (`self.Pickups`) 1))
    (set `self.Attempts` (`self.Pickups`))
    (set `self.NextTime` (+ _returnvalue (`KismetMathLibrary.RandomFloatInRange` 1.5 3.5))))
  (set `self.LastCarry` _carrying)
  (if (== (`self.Mode`) 0)
    (`SceneComponent.SetVisibility` (`self.Model`) false true)
    (set `self.Warn` false)
    (if (and (and (== _state 1) (> _carrying 0)) (and (> (`self.Attempts`) 0) (> _returnvalue (`self.NextTime`))))
      (set `self.Attempts` (- (`self.Attempts`) 1))
      (bind _returnvalue_7 (`self.K2_GetActorLocation` _asbp_nyc_pigeon))
      (set `self.P0` (`KismetMathLibrary.MakeVector` (+ (.x _returnvalue_7) (* (select `bool` (`KismetMathLibrary.RandomBool`) :`false` -1.0 :`true` 1.0) 1600.0)) (- (.y _returnvalue_7) 500.0) 900.0))
      (set `self.P1` _returnvalue_7)
      (set `self.T` 0.0)
      (set `self.Mode` 1)
      (set `self.Warn` true)
      (`self.K2_SetActorLocation` self (`self.P0`) false true)
      (`SceneComponent.SetVisibility` (`self.Model`) true true))
    (elif (== (`self.Mode`) 1)
      (set `self.T` _returnvalue_5)
      (bind _returnvalue_8 (+ (`KismetMathLibrary.VLerp` (`self.P0`) (+ (`KismetMathLibrary.VLerp` (`self.P1`) _returnvalue_7 0.35) (`KismetMathLibrary.MakeVector` 0.0 0.0 25.0)) _returnvalue_5) (`KismetMathLibrary.MakeVector` 0.0 0.0 (* (`KismetMathLibrary.DegSin` (* _returnvalue_5 180.0)) 120.0))))
      (`self.K2_SetActorLocation` self _returnvalue_8 false true)
      (`self.K2_SetActorRotation` self (`KismetMathLibrary.MakeRotator` (* _returnvalue_3 8.0) -10.0 (`KismetMathLibrary.DegAtan2` (- (.y _returnvalue_8) (.y _returnvalue_2)) (- (.x _returnvalue_8) (.x _returnvalue_2)))) true)
      (if (>= _returnvalue_5 1.0)
        (set `self.P1` (+ _returnvalue_8 (`KismetMathLibrary.MakeVector` (* (- (.x _returnvalue_8) (.x (`self.P0`))) 1.5) 2200.0 1100.0)))
        (set `self.P0` _returnvalue_8)
        (set `self.T` 0.0)
        (set `self.Mode` 2)
        (set `self.Warn` false)
        (if (and (< (`KismetMathLibrary.Sqrt` (+ (* (- (.x _returnvalue_8) (.x _returnvalue_7)) (- (.x _returnvalue_8) (.x _returnvalue_7))) (* (- (.y _returnvalue_8) (.y _returnvalue_7)) (- (.y _returnvalue_8) (.y _returnvalue_7))))) 130.0) (> _carrying 0))
          (set `self.HasFood` _carrying)
          (`/Game/NYCrossing/Blueprints/BP_NYC_Pigeon.Steal` _asbp_nyc_pigeon)
          (`SceneComponent.SetVisibility` _food true true)
          (switch `int` _carrying
            (:`1`
              (`StaticMeshComponent.SetStaticMesh` _food "/Game/NYCrossing/Assets3D/HotDog/SM_HotDog_cm.SM_HotDog_cm"))
            (:`2`
              (`StaticMeshComponent.SetStaticMesh` _food "/Game/NYCrossing/Assets3D/Pizza/SM_Pizza_cm.SM_Pizza_cm"))
            (:`3`
              (`StaticMeshComponent.SetStaticMesh` _food "/Game/NYCrossing/Assets3D/Cheesecake/SM_Cheesecake_cm.SM_Cheesecake_cm"))
            (:`4`
              (`StaticMeshComponent.SetStaticMesh` _food "/Game/NYCrossing/Assets3D/Soda/SM_Soda_cm.SM_Soda_cm")))))
      (elif (== (`self.Mode`) 2)
        (set `self.T` _returnvalue_4)
        (`self.K2_SetActorLocation` self _returnvalue_6 false true)
        (`self.K2_SetActorRotation` self (`KismetMathLibrary.MakeRotator` (* _returnvalue_3 8.0) 15.0 (`KismetMathLibrary.DegAtan2` (- (.y _returnvalue_6) (.y _returnvalue_2)) (- (.x _returnvalue_6) (.x _returnvalue_2)))) true)
        (if (>= _returnvalue_4 1.0)
          (set `self.Mode` 0)
          (set `self.HasFood` 0)
          (`SceneComponent.SetVisibility` _food false true)
          (set `self.NextTime` (+ _returnvalue (`KismetMathLibrary.RandomFloatInRange` 2.5 4.5))))))))

(fn `UserConstructionScript`)