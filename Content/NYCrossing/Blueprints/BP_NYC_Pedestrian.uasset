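; Pedestrian in NYCrossing that walks back and forth along Y in a lane snapped to an X grid, killing pigeons in its path.
; BeginPlay picks a random side, then Tick alternates timed random waits with crossings, re-randomizing the X offset before each and turning around at the far end.
; Movement is teleport-based with sine-swung hip pivots, and pigeon hits are distance checks on low-altitude BP_NYC_Pigeon actors.
; An older, unconnected copy of the walk logic remains.
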(event `self.ReceiveBeginPlay`
  (set `self.BaseX` (* (`KismetMathLibrary.Round` (/ (.x (`self.K2_GetActorLocation`)) 1500.0)) 1500.0))
  (set `self.Dir` (select `bool` (`KismetMathLibrary.RandomBool`) :`false` -1.0 :`true` 1.0))
  (`self.K2_SetActorLocation` self (`KismetMathLibrary.MakeVector` (+ (`self.BaseX`) (`KismetMathLibrary.RandomFloatInRange` -200.0 200.0)) (* (- 0.0 (`self.Dir`)) 2050.0) 10.0) false true)
  (`self.K2_SetActorRotation` self (`KismetMathLibrary.MakeRotator` 0.0 0.0 (select `bool` (> (`self.Dir`) 0.0) :`false` -90.0 :`true` 90.0)) false)
  (set `self.Walking` false)
  (set `self.WaitUntil` (+ (`KismetSystemLibrary.GetGameTimeInSeconds`) (`KismetMathLibrary.RandomFloatInRange` 0.0 8.0))))

(event `self.ReceiveTick`
  (params (DeltaSeconds :type "Float (single-precision)"))
  (bind _returnvalue (`KismetSystemLibrary.GetGameTimeInSeconds`))
  (bind _returnvalue_2 (`self.K2_GetActorLocation`))
  (bind _returnvalue_3 (* (`KismetMathLibrary.DegSin` (* _returnvalue 500.0)) 25.0))
  (bind _returnvalue_4 (+ (.y _returnvalue_2) (* (`self.Dir`) (* (`self.Speed`) DeltaSeconds))))
  (if (`self.Walking`)
    (`self.K2_SetActorLocation` self (`KismetMathLibrary.MakeVector` (.x _returnvalue_2) _returnvalue_4 10.0) false true)
    (`SceneComponent.K2_SetRelativeRotation` (`self.HipL`) (`KismetMathLibrary.MakeRotator` 0.0 _returnvalue_3) false false)
    (`SceneComponent.K2_SetRelativeRotation` (`self.HipR`) (`KismetMathLibrary.MakeRotator` 0.0 (- 0.0 _returnvalue_3)) false false)
    (bind _outactors (`GameplayStatics.GetAllActorsOfClass` "/Game/NYCrossing/Blueprints/BP_NYC_Pigeon.BP_NYC_Pigeon_C"))
    (for _array_element _outactors
      (bind _returnvalue_5 (`self.K2_GetActorLocation` _array_element))
      (if (and (< (`KismetMathLibrary.Abs` (- (.x _returnvalue_5) (.x _returnvalue_2))) 55.0) (and (< (`KismetMathLibrary.Abs` (- (.y _returnvalue_5) _returnvalue_4)) 55.0) (< (.z _returnvalue_5) 100.0)))
        (`/Game/NYCrossing/Blueprints/BP_NYC_Pigeon.Die` _array_element)))
    (if (> (* (`self.Dir`) _returnvalue_4) 2050.0)
      (set `self.Walking` false)
      (set `self.WaitUntil` (+ _returnvalue (`KismetMathLibrary.RandomFloatInRange` 3.0 11.0)))
      (set `self.Dir` (- 0.0 (`self.Dir`)))
      (`SceneComponent.K2_SetRelativeRotation` (`self.HipL`) (`KismetMathLibrary.MakeRotator` 0.0) false false)
      (`SceneComponent.K2_SetRelativeRotation` (`self.HipR`) (`KismetMathLibrary.MakeRotator` 0.0) false false)
      (`self.K2_SetActorRotation` self (`KismetMathLibrary.MakeRotator` 0.0 0.0 (select `bool` (> (`self.Dir`) 0.0) :`false` -90.0 :`true` 90.0)) false))
    (elif (> _returnvalue (`self.WaitUntil`))
      (set `self.Walking` true)
      (`self.K2_SetActorLocation` self (`KismetMathLibrary.MakeVector` (+ (`self.BaseX`) (`KismetMathLibrary.RandomFloatInRange` -200.0 200.0)) (.y _returnvalue_2) 10.0) false true))))

(fn `UserConstructionScript`)