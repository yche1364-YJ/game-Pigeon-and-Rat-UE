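; A pedestrian crossing signal for the NYCrossing scene that cycles through walk, flashing countdown and don't-walk phases.
; Each Tick derives the phase from game time modulo the cycle length, so the timing needs no timers or stored start time.
; It sets State and Countdown, swaps the lamp between green and orange materials, blinks it during the flash phase, and updates the text to WALK, seconds left, or DONT WALK.
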(event `self.ReceiveTick`
  (params (DeltaSeconds :type "Float (single-precision)"))
  (bind _returnvalue (`KismetSystemLibrary.GetGameTimeInSeconds`))
  (bind _cyclelength (`self.CycleLength`))
  (bind _walktime (`self.WalkTime`))
  (bind _lamp (`self.Lamp`))
  (bind _signaltext (`self.SignalText`))
  (bind _returnvalue_2 (mod _returnvalue _cyclelength))
  (bind _returnvalue_3 (+ _walktime (`self.FlashTime`)))
  (bind _returnvalue_4 (`KismetMathLibrary.FCeil` (- _returnvalue_3 _returnvalue_2)))
  (if (< _returnvalue_2 _walktime)
    (set `self.State` 0)
    (set `self.Countdown` (`KismetMathLibrary.FCeil` (- _walktime _returnvalue_2)))
    (`PrimitiveComponent.SetMaterial` _lamp 0 "/Game/NYCrossing/Materials/MI_Green.MI_Green")
    (`SceneComponent.SetVisibility` _lamp true false)
    (`TextRenderComponent.K2_SetText` _signaltext (`KismetTextLibrary.Conv_StringToText` "WALK"))
    (elif (< _returnvalue_2 _returnvalue_3)
      (set `self.State` 1)
      (set `self.Countdown` _returnvalue_4)
      (`PrimitiveComponent.SetMaterial` _lamp 0 "/Game/NYCrossing/Materials/MI_Orange.MI_Orange")
      (`SceneComponent.SetVisibility` _lamp (< (`KismetMathLibrary.Fraction` (* _returnvalue 2.0)) 0.5) false)
      (`TextRenderComponent.K2_SetText` _signaltext (`KismetTextLibrary.Conv_IntToText` _returnvalue_4))
      (else
        (set `self.State` 2)
        (set `self.Countdown` (`KismetMathLibrary.FCeil` (- _cyclelength _returnvalue_2)))
        (`PrimitiveComponent.SetMaterial` _lamp 0 "/Game/NYCrossing/Materials/MI_Orange.MI_Orange")
        (`SceneComponent.SetVisibility` _lamp true false)
        (`TextRenderComponent.K2_SetText` _signaltext (`KismetTextLibrary.Conv_StringToText` "DONT WALK"))))))

(fn `UserConstructionScript`)