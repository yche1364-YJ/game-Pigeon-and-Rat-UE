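; BP_NYC_Rat is a rat actor for NYCrossing, with its construction script as the only active logic.
; The script hides bird-shaped components (body, neck, head, beak, tail, both wings), which suggests they come from a shared bird base.
; It also hides the CarryDog and CarryPizza components along with their children.
; Its event graph holds only disabled stubs, so this graph adds no runtime behavior.
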(fn `UserConstructionScript`
  (`SceneComponent.SetVisibility` (`self.Body`) false false)
  (`SceneComponent.SetVisibility` (`self.Neck`) false false)
  (`SceneComponent.SetVisibility` (`self.Head`) false false)
  (`SceneComponent.SetVisibility` (`self.Beak`) false false)
  (`SceneComponent.SetVisibility` (`self.Tail`) false false)
  (`SceneComponent.SetVisibility` (`self.WingL`) false false)
  (`SceneComponent.SetVisibility` (`self.WingR`) false false)
  (`SceneComponent.SetVisibility` (`self.CarryDog`) false true)
  (`SceneComponent.SetVisibility` (`self.CarryPizza`) false true))