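; BP_NYC_PizzaBench is a food pickup for NYCrossing, showing a spinning hot dog, pizza, cheesecake or soda on an optionally visible bench.
; SetupFood picks FoodMesh's mesh and height from FoodType, in both the construction script and BeginPlay.
; Take, which has no caller here, hides the food and sets a random respawn time that Tick polls to show it again.
; ShowFood toggles FoodMesh and always hides PizzaRoot and HotDogRoot.
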(event `self.ReceiveBeginPlay`
  (set `self.Available` true)
  (`SceneComponent.SetVisibility` (`self.BenchRoot`) (`self.ShowBench`) true)
  (`self.SetupFood`)
  (`self.ShowFood` true))

(event `self.ReceiveTick`
  (params (DeltaSeconds :type "Float (single-precision)"))
  (`SceneComponent.K2_AddLocalRotation` (`self.FoodMesh`) (`KismetMathLibrary.MakeRotator` 0.0 0.0 (* DeltaSeconds 70.0)) false false)
  (if (and (not (`self.Available`)) (> (`KismetSystemLibrary.GetGameTimeInSeconds`) (`self.RespawnAt`)))
    (set `self.Available` true)
    (`self.ShowFood` true)))

(fn `SetupFood`
  (bind _foodmesh (`self.FoodMesh`))
  (bind _foodtype (`self.FoodType`))
  (`SceneComponent.K2_SetRelativeLocation` _foodmesh (`KismetMathLibrary.MakeVector` 0.0 -5.0 (select `bool` (== _foodtype 1) :`false` 62.0 :`true` 6.0)) false false)
  (switch `int` (- _foodtype 1)
    (:`0`
      (`StaticMeshComponent.SetStaticMesh` _foodmesh "/Game/NYCrossing/Assets3D/HotDog/SM_HotDog_cm.SM_HotDog_cm"))
    (:`1`
      (`StaticMeshComponent.SetStaticMesh` _foodmesh "/Game/NYCrossing/Assets3D/Pizza/SM_Pizza_cm.SM_Pizza_cm"))
    (:`2`
      (`StaticMeshComponent.SetStaticMesh` _foodmesh "/Game/NYCrossing/Assets3D/Cheesecake/SM_Cheesecake_cm.SM_Cheesecake_cm"))
    (:`3`
      (`StaticMeshComponent.SetStaticMesh` _foodmesh "/Game/NYCrossing/Assets3D/Soda/SM_Soda_cm.SM_Soda_cm"))))

(fn `ShowFood`
  (params (Vis :type Boolean))
  (`SceneComponent.SetVisibility` (`self.PizzaRoot`) false true)
  (`SceneComponent.SetVisibility` (`self.HotDogRoot`) false true)
  (`SceneComponent.SetVisibility` (`self.FoodMesh`) Vis true))

(fn `Take`
  (set `self.Available` false)
  (set `self.RespawnAt` (+ (`KismetSystemLibrary.GetGameTimeInSeconds`) (`KismetMathLibrary.RandomFloatInRange` 3.0 6.0)))
  (`self.ShowFood` false))

(fn `UserConstructionScript`
  (`SceneComponent.SetVisibility` (`self.BenchRoot`) (`self.ShowBench`) true)
  (`self.SetupFood`)
  (`self.ShowFood` true))