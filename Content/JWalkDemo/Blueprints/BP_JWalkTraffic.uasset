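; Traffic vehicle for the JWalk demo that drives along its lane and catches a pedestrian player who steps into its path.
; Each Tick derives position statelessly from game time, Direction, Offset and Lane: looping along X during the first part of a repeating cycle, then waiting at one end.
; A distance-box test replaces collision: a hit teleports the player back to a fixed start and sends BP_JWalkDirector a timed warning about van-hidden traffic.
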(event `self.ReceiveTick`
  (params (DeltaSeconds :type "Float (single-precision)"))
  (bind _returnvalue (`KismetSystemLibrary.GetGameTimeInSeconds`))
  (bind _returnvalue_2 (`GameplayStatics.GetPlayerCharacter` 0))
  (bind _lane (`self.Lane`))
  (bind _returnvalue_3 (mod _returnvalue 20.0))
  (bind _returnvalue_4 (`self.K2_GetActorLocation` _returnvalue_2))
  (bind _returnvalue_5 (* (`self.Direction`) (select `bool` (< _returnvalue_3 8.0) :`false` 3800.0 :`true` (- (* (mod (+ _returnvalue_3 (`self.Offset`)) 8.0) 900.0) 3600.0))))
  (`self.K2_SetActorLocation` self (`KismetMathLibrary.MakeVector` _returnvalue_5 _lane) false false)
  (if (and (< (`KismetMathLibrary.Abs` (- (.x _returnvalue_4) _returnvalue_5)) 270.0) (and (< (`KismetMathLibrary.Abs` (- (.y _returnvalue_4) _lane)) 145.0) (< (.z _returnvalue_4) 270.0)))
    (`KismetSystemLibrary.PrintString` "CLOSE CALL! A stopped van can hide moving traffic. Look across EVERY lane." true false (struct :`G` 0.66 :`B` 1.0 :`A` 1.0) 4.0 "JWalkFeedback")
    (`self.K2_SetActorLocation` _returnvalue_2 (`KismetMathLibrary.MakeVector` 0.0 -1200.0 120.0) false true)
    (bind _returnvalue_6 (`GameplayStatics.GetActorOfClass` "/Game/JWalkDemo/Blueprints/BP_JWalkDirector.BP_JWalkDirector_C"))
    (bind _asbp_jwalk_director (cast `/Game/JWalkDemo/Blueprints/BP_JWalkDirector` _returnvalue_6))
    (set `/Game/JWalkDemo/Blueprints/BP_JWalkDirector.Feedback` "CLOSE CALL: the van hid traffic. Check EVERY lane." _asbp_jwalk_director)
    (set `/Game/JWalkDemo/Blueprints/BP_JWalkDirector.FeedbackUntil` (+ _returnvalue 5.0) _asbp_jwalk_director)))

(fn `UserConstructionScript`)