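; Director for the JWalk demo, a pedestrian crossing challenge that assigns the HUD and drives two WAIT/WALK signal texts.
; Tick derives a 20-second, half-WAIT, half-WALK cycle from game time and flags the player Risky when in the road during WAIT.
; Reaching the far-side goal sets Completed, or if Risky, sets timed feedback and teleports the player to the start.
; Falling or leaving the bounds also teleports to the start.
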(event `self.ReceiveBeginPlay`
  (`KismetSystemLibrary.DelayUntilNextTick`)
  (`PlayerController.ClientSetHUD` (`GameplayStatics.GetPlayerController` 0) "/Game/JWalkDemo/Blueprints/BP_JWalkHUD.BP_JWalkHUD_C"))

(event `self.ReceiveTick`
  (params (DeltaSeconds :type "Float (single-precision)"))
  (bind _returnvalue (`KismetSystemLibrary.GetGameTimeInSeconds`))
  (bind _returnvalue_2 (`GameplayStatics.GetPlayerCharacter` 0))
  (bind _returnvalue_3 (mod _returnvalue 20.0))
  (bind _returnvalue_4 (`self.K2_GetActorLocation` _returnvalue_2))
  (bind _returnvalue_5 (select `bool` (>= _returnvalue_3 10.0) :`false` "WAIT" :`true` "WALK"))
  (`TextRenderComponent.K2_SetText` (`self.SignalNear`) (`KismetTextLibrary.Conv_StringToText` _returnvalue_5))
  (`TextRenderComponent.K2_SetText` (`self.SignalFar`) (`KismetTextLibrary.Conv_StringToText` _returnvalue_5))
  (if (< (.y _returnvalue_4) -900.0)
    (set `self.Risky` false))
  (if (and (< _returnvalue_3 10.0) (and (> (.y _returnvalue_4) -780.0) (< (.y _returnvalue_4) 780.0)))
    (set `self.Risky` true))
  (if (and (> (.y _returnvalue_4) 1000.0) (< (`KismetMathLibrary.Abs` (.x _returnvalue_4)) 280.0))
    (if (`self.Risky`)
      (set `self.Feedback` "WAIT crossing: arrival was luck. Try a safe crossing.")
      (set `self.FeedbackUntil` (+ _returnvalue 5.0))
      (`self.K2_SetActorLocation` _returnvalue_2 (`KismetMathLibrary.MakeVector` 0.0 -1200.0 120.0) false true)
      (else
        (set `self.Completed` true))))
  (if (or (< (.z _returnvalue_4) -100.0) (or (> (`KismetMathLibrary.Abs` (.x _returnvalue_4)) 2900.0) (> (`KismetMathLibrary.Abs` (.y _returnvalue_4)) 1400.0)))
    (`self.K2_SetActorLocation` _returnvalue_2 (`KismetMathLibrary.MakeVector` 0.0 -1200.0 120.0) false true)))

(fn `UserConstructionScript`)