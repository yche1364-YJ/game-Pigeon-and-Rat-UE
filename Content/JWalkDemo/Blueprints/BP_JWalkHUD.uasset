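; HUD for the J/Walk street-safety prototype, drawn in immediate mode from DrawHUD with rects and text.
; It shows a title panel whose WALK/WAIT signal, hint and accent color alternate on game time modulo a fixed cycle, plus a bottom controls and goal bar.
; It looks up BP_JWalkDirector every frame to show timed feedback and a completion panel.
; An unconnected, smaller-text copy of the drawing chain never runs.
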(event `self.ReceiveDrawHUD`
  (params (SizeX :type Integer) (SizeY :type Integer))
  (bind _returnvalue (`KismetSystemLibrary.GetGameTimeInSeconds`))
  (bind _linearcolor (make `LinearColor` 0.95 0.96 0.93 1.0))
  (bind _linearcolor_2 (make `LinearColor` 1.0 0.63 0.15 1.0))
  (bind _linearcolor_3 (make `LinearColor` 0.18 0.95 0.62 1.0))
  (bind _linearcolor_4 (make `LinearColor` 0.018 0.028 0.045 0.88))
  (bind _returnvalue_2 (>= (mod _returnvalue 20.0) 10.0))
  (`self.DrawRect` _linearcolor_4 20.0 20.0 590.0 154.0)
  (`self.DrawRect` (select `bool` _returnvalue_2 :`false` _linearcolor_2 :`true` _linearcolor_3) 20.0 20.0 5.0 154.0)
  (`self.DrawText` "J / WALK" _linearcolor 40.0 30.0 null 3.0)
  (`self.DrawText` "NEW YORK  /  STREET SAFETY PROTOTYPE" _linearcolor_2 40.0 65.0 null 1.6)
  (`self.DrawText` (select `bool` _returnvalue_2 :`false` "WAIT - TRAFFIC HAS THE ROAD" :`true` "WALK - CHECK BOTH LANES") (select `bool` _returnvalue_2 :`false` _linearcolor_2 :`true` _linearcolor_3) 40.0 91.0 null 1.8)
  (`self.DrawText` (select `bool` _returnvalue_2 :`false` "A stopped delivery van can hide a moving car." :`true` "Reach the green pad. Stay alert even with WALK.") _linearcolor 40.0 125.0 null 1.6)
  (`self.DrawRect` _linearcolor_4 20.0 (- SizeY 74.0) 590.0 54.0)
  (`self.DrawText` "WASD  Move     MOUSE  Look     ESC  Stop" _linearcolor 40.0 (- SizeY 61.0) null 1.6)
  (`self.DrawText` "Goal: cross safely to the GREEN arrival pad." _linearcolor_2 40.0 (- SizeY 42.0) null 1.6)
  (bind _returnvalue_3 (`GameplayStatics.GetActorOfClass` "/Game/JWalkDemo/Blueprints/BP_JWalkDirector.BP_JWalkDirector_C"))
  (bind _asbp_jwalk_director (cast `/Game/JWalkDemo/Blueprints/BP_JWalkDirector` _returnvalue_3))
  (if (< _returnvalue (`/Game/JWalkDemo/Blueprints/BP_JWalkDirector.FeedbackUntil` _asbp_jwalk_director))
    (`self.DrawRect` _linearcolor_4 20.0 190.0 720.0 65.0)
    (`self.DrawText` (`/Game/JWalkDemo/Blueprints/BP_JWalkDirector.Feedback` _asbp_jwalk_director) _linearcolor_2 40.0 208.0 null 1.1))
  (if (`/Game/JWalkDemo/Blueprints/BP_JWalkDirector.Completed` _asbp_jwalk_director)
    (`self.DrawRect` _linearcolor_4 20.0 275.0 590.0 90.0)
    (`self.DrawText` "SAFE ARRIVAL" _linearcolor_3 40.0 290.0 null 2.0)
    (`self.DrawText` "You waited and crossed safely. ESC, then Play to retry." _linearcolor 40.0 333.0 null 1.6)))

(fn `UserConstructionScript`)